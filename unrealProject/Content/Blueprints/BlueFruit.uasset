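; Blue fruit physics actor that alternates between cutting and merging whenever its glow flag is set.
; While glowing, Tick scales the mesh and a FlipFlop plays or reverses a timeline driving its material Blend.
; After a cut it hides and teleports every CutBlueFruit to itself, revealed and glowing; after a merge it restores physics and collision.
; When not glowing, it applies a velocity-based buoyancy force inside overlaps named PhysicsVolume.
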(event `self.ReceiveHit`
  (params (MyComp :type "PrimitiveComponent Object Reference") (Other :type "Actor Object Reference") (OtherComp :type "PrimitiveComponent Object Reference") (bSelfMoved :type Boolean) (HitLocation :type "Vector Structure") (HitNormal :type "Vector Structure") (NormalImpulse :type "Vector Structure") (Hit :type "HitResult Structure (by ref)"))
  (if (`KismetMathLibrary.ClassIsChildOf` (`GameplayStatics.GetObjectClass` Other) "/Game/SideScrollerCPP/Blueprints/SideScrollerCharacter2.SideScrollerCharacter2_C")
    _))

(event `self.ReceiveTick`
  (params (DeltaSeconds :type "Float (single-precision)"))
  (bind _staticmeshcomponent (`self.StaticMeshComponent`))
  (bind _staticmeshcomponent_2 (`self.StaticMeshComponent`))
  (bind _staticmeshcomponent_3 (`self.StaticMeshComponent`))
  (bind _returnvalue (`SceneComponent.K2_GetComponentScale` _staticmeshcomponent_3))
  (bind _returnvalue_2 (`SceneComponent.K2_GetComponentScale` _staticmeshcomponent_3))
  (if (`SceneComponent.IsVisible` (`self.StaticMeshComponent`))
    (if (`self.IsGlow`)
      (`PrimitiveComponent.SetSimulatePhysics` _staticmeshcomponent false)
      (`PrimitiveComponent.SetCollisionResponseToChannel` _staticmeshcomponent "ECC_Pawn" "ECR_Block")
      (`|ExecutionSequence`
        (:`then_0`
          ;[1 1 1] Shrink Berry
          (if (`self.shouldShrink`)
            (if (`KismetMathLibrary.InRange_FloatFloat` (.x _returnvalue) 3.5 4.0)
              (set `self.shouldShrink` false)
              (else
                (`SceneComponent.SetWorldScale3D` (`self.StaticMeshComponent`) (- _returnvalue (0.05 0.05 0.05)))))))
        (:`then_1`
          ;[1 1 1] Growing
          (if (`self.shouldGrow`)
            _
            (elif (`KismetMathLibrary.InRange_FloatFloat` (.x _returnvalue_2) 8.5 8.6)
              (set `self.shouldGrow` false)
              (else
                (`SceneComponent.SetWorldScale3D` _staticmeshcomponent_3 (+ _returnvalue_2 (0.05 0.05 0.05)))))))
        (:`then_2`
          (if (not (`self.calledOnce`))
            (set `self.calledOnce` true)
            (bind _isa (`/Engine/EditorBlueprintResources/StandardMacros.FlipFlop`)
              (:`A`
                (bind (_direction _blend) (`Timeline|Timeline_0` :!via `PlayFromStart` :!label _label)
                  (:`Update`
                    (set `self.shouldGrow` _isa)
                    (`MeshComponent.SetScalarParameterValueOnMaterials` (`self.StaticMeshComponent`) "Blend" _blend))
                  (:`Finished`
                    (set `self.IsGlow` false)
                    (set `self.calledOnce` false)
                    (if _isa
                      ;[1 1 1] After cut
                      (`PrimitiveComponent.SetSimulatePhysics` _staticmeshcomponent_2 false)
                      (`PrimitiveComponent.SetCollisionResponseToChannel` _staticmeshcomponent_2 "ECC_PhysicsBody" "ECR_Ignore")
                      (`PrimitiveComponent.SetCollisionResponseToChannel` _staticmeshcomponent_2 "ECC_Pawn" "ECR_Ignore")
                      (`SceneComponent.SetVisibility` _staticmeshcomponent_2 false false)
                      (bind _outactors (`GameplayStatics.GetAllActorsOfClass` "/Game/Blueprints/cutBlueFruit.cutBlueFruit_C"))
                      (for _array_element _outactors
                        (`self.K2_SetActorLocation` _array_element (`self.K2_GetActorLocation`) false true)
                        (`SceneComponent.SetVisibility` (`StaticMeshActor.StaticMeshComponent` _array_element) true false)
                        (set `/Game/Blueprints/cutBlueFruit.IsGlowSmall` true _array_element))
                      (else
                        ;[1 1 1] After merge
                        (`PrimitiveComponent.SetSimulatePhysics` _staticmeshcomponent_2 true)
                        (`PrimitiveComponent.SetCollisionResponseToChannel` _staticmeshcomponent_2 "ECC_Pawn" "ECR_Block")
                        (`PrimitiveComponent.SetCollisionResponseToChannel` _staticmeshcomponent_2 "ECC_PhysicsBody" "ECR_Block"))))))
              (:`B`
                (goto _label :!via `ReverseFromEnd`))))))
      (else
        ;[1 1 1] Update buyancy water force
        (if (`self.inWater`)
          (`PrimitiveComponent.AddForce` (`self.StaticMeshComponent`) (`KismetMathLibrary.MakeVector` (.x (`self.GetVelocity`)) (.y (`self.GetVelocity`)) (- (.z (`self.GetVelocity`)) (`self.Buyancy`))) "None" false))))))

(event `self.ReceiveBeginPlay`
  (bind _staticmeshcomponent (`self.StaticMeshComponent`))
  (`PrimitiveComponent.CreateDynamicMaterialInstance` _staticmeshcomponent 0 (`PrimitiveComponent.GetMaterial` _staticmeshcomponent 0)))

(event `self.ReceiveActorBeginOverlap`
  (params (OtherActor :type "Actor Object Reference"))
  ;[1 1 1] Berry Hits water
  (`KismetSystemLibrary.PrintString` (`KismetSystemLibrary.GetDisplayName` OtherActor))
  (if (`KismetStringLibrary.EqualEqual_StrStr` (`KismetSystemLibrary.GetDisplayName` OtherActor) "PhysicsVolume")
    (set `self.inWater` true)
    (`PrimitiveComponent.AddForce` (`self.StaticMeshComponent`) (`KismetMathLibrary.MakeVector` (.x (`self.GetVelocity`)) (.y (`self.GetVelocity`)) (- (.z (`self.GetVelocity`)) (`self.Buyancy`))) "None" false)))

(event `self.ReceiveActorEndOverlap`
  (params (OtherActor :type "Actor Object Reference"))
  ;[1 1 1] Berry Hits water
  (if (`KismetStringLibrary.EqualEqual_StrStr` (`KismetSystemLibrary.GetDisplayName` OtherActor) "PhysicsVolume")
    (`PrimitiveComponent.SetEnableGravity` (`self.StaticMeshComponent`) true)
    (set `self.inWater` false)))

(fn `Glow`)

(fn `UserConstructionScript`)
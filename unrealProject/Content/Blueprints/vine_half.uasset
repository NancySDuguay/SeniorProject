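; Vine half actor that can highlight its static mesh when the player is nearby.
; The Highlight function enables Custom Depth rendering on the mesh when the first player's pawn is within a short fixed distance, and disables it otherwise.
; Its event graph and construction script are empty, so nothing in this Blueprint calls Highlight.
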(event `self.ReceiveTick`
  (params (DeltaSeconds :type "Float (single-precision)")))

(fn `Highlight`
  (if (<= (`KismetMathLibrary.VSize` (- (`self.K2_GetActorLocation` (`GameplayStatics.GetPlayerPawn` 0)) (`self.K2_GetActorLocation`))) 200.0)
    (`PrimitiveComponent.SetRenderCustomDepth` (`self.StaticMeshComponent`) true)
    (else
      (`PrimitiveComponent.SetRenderCustomDepth` (`self.StaticMeshComponent`) false))))

(fn `UserConstructionScript`)
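; Lotus collectible that spins every tick and is picked up when player character 0 or 1 overlaps it.
; On overlap it destroys itself and increments LotusCount on NewGameState.
; It then shows a LotusFlower popup in Game and UI input mode, or removes it if LotusUI is already valid.
; A four-second Delay precedes restoring game-only input, but it follows DestroyActor on the same actor.
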(event `self.ReceiveActorBeginOverlap`
  (params (OtherActor :type "Actor Object Reference"))
  (bind _lotusui (`self.LotusUI`))
  (if (or (== OtherActor (`GameplayStatics.GetPlayerCharacter` 0)) (== OtherActor (`GameplayStatics.GetPlayerCharacter` 1)))
    (`self.K2_DestroyActor`)
    (bind _asnew_game_state (cast `/Game/Blueprints/NewGameState` (`GameplayStatics.GetGameState`)))
    (set `/Game/Blueprints/NewGameState.lotusCount` (+ (`/Game/Blueprints/NewGameState.lotusCount` _asnew_game_state) 1) _asnew_game_state)
    ;[1 1 1] Lotus UI Pop Up
    (`/Engine/EditorBlueprintResources/StandardMacros.IsValid` (`self.LotusUI`)
      (:`Is Valid`
        (`Widget.RemoveFromParent` (stale _returnvalue)))
      (:`Is Not Valid`
        (bind _returnvalue (`|CreateWidget` "/Game/UI/lotusFlower.lotusFlower_C"))
        (set `self.LotusUI` _returnvalue)
        (`WidgetBlueprintLibrary.SetInputMode_GameAndUIEx` (`GameplayStatics.GetPlayerController` 0) _lotusui)
        (`UserWidget.AddToViewport` _lotusui 0)
        (`KismetSystemLibrary.Delay` 4.0)
        (`WidgetBlueprintLibrary.SetInputMode_GameOnly` (`GameplayStatics.GetPlayerController` 0))
        (`WidgetBlueprintLibrary.SetInputMode_GameOnly` (`GameplayStatics.GetPlayerController` 1))))))

(event `self.ReceiveTick`
  (params (DeltaSeconds :type "Float (single-precision)"))
  (`self.K2_AddActorLocalRotation` (struct :`Yaw` 3.0)))

(fn `UserConstructionScript`)
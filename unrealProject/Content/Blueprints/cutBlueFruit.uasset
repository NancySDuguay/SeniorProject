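; Cut blue fruit actor with simple water physics and a proximity highlight.
; Overlapping an actor named PhysicsVolume sets InWater and applies a force built from velocity with Buyancy subtracted from Z, repeated each Tick.
; Leaving clears InWater and enables gravity, though the node disabling gravity is unconnected.
; Highlight, not called within this Blueprint, toggles custom depth rendering by player pawn distance.
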(event `self.ReceiveActorBeginOverlap`
  (params (OtherActor :type "Actor Object Reference"))
  (if (`KismetStringLibrary.EqualEqual_StrStr` (`KismetSystemLibrary.GetDisplayName` OtherActor) "PhysicsVolume")
    (set `self.inWater` true)
    (`PrimitiveComponent.AddForce` (`self.StaticMeshComponent`) (`KismetMathLibrary.MakeVector` (.x (`self.GetVelocity`)) (.y (`self.GetVelocity`)) (- (.z (`self.GetVelocity`)) (`self.Buyancy`))) "None" false)))

(event `self.ReceiveTick`
  (params (DeltaSeconds :type "Float (single-precision)"))
  (if (`self.inWater`)
    (`PrimitiveComponent.AddForce` (`self.StaticMeshComponent`) (`KismetMathLibrary.MakeVector` (.x (`self.GetVelocity`)) (.y (`self.GetVelocity`)) (- (.z (`self.GetVelocity`)) (`self.Buyancy`))) "None" false)))

(event `self.ReceiveActorEndOverlap`
  (params (OtherActor :type "Actor Object Reference"))
  (if (`KismetStringLibrary.EqualEqual_StrStr` (`KismetSystemLibrary.GetDisplayName` OtherActor) "PhysicsVolume")
    (`PrimitiveComponent.SetEnableGravity` (`self.StaticMeshComponent`) true)
    (set `self.inWater` false)))

(fn `Highlight`
  (if (<= (`KismetMathLibrary.VSize` (- (`self.K2_GetActorLocation` (`GameplayStatics.GetPlayerPawn` 0)) (`self.K2_GetActorLocation`))) 150.0)
    (`PrimitiveComponent.SetRenderCustomDepth` (`self.StaticMeshComponent`) true)
    (else
      (`PrimitiveComponent.SetRenderCustomDepth` (`self.StaticMeshComponent`) false))))

(fn `UserConstructionScript`)
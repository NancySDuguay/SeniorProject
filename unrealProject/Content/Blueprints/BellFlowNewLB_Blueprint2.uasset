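; A bell flower actor that grows to its start scale and, when touched by SideScrollerCharacter2, falls while spinning.
; Once below a height threshold, it shrinks and a timeline drives the material's Blend parameter.
; Overlapping another bell flower or a non-character actor stops it and spawns a successor at its origin with GrowNum decremented, or a VineBud at zero.
; Stopped flowers creep upward and enlarge to a capped size.
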(event `self.ReceiveBeginPlay`
  (bind _staticmesh (`self.StaticMesh`))
  (`PrimitiveComponent.CreateDynamicMaterialInstance` _staticmesh 0 (`PrimitiveComponent.GetMaterial` _staticmesh 0))
  (set `self.startLoc` (`self.K2_GetActorLocation`))
  (set `self.onGrow` true)
  (set `self.onHit` false)
  (set `self.startScale` (`self.GetActorScale3D`)))

(event `self.ReceiveHit`
  (params (MyComp :type "PrimitiveComponent Object Reference") (Other :type "Actor Object Reference") (OtherComp :type "PrimitiveComponent Object Reference") (bSelfMoved :type Boolean) (HitLocation :type "Vector Structure") (HitNormal :type "Vector Structure") (NormalImpulse :type "Vector Structure") (Hit :type "HitResult Structure (by ref)")))

(event `self.Box.OnComponentBeginOverlap`
  (params (OverlappedComponent :type "PrimitiveComponent Object Reference") (OtherActor :type "Actor Object Reference") (OtherComp :type "PrimitiveComponent Object Reference") (OtherBodyIndex :type Integer) (bFromSweep :type Boolean) (SweepResult :type "HitResult Structure (by ref)")))

(event `self.ReceiveActorBeginOverlap`
  (params (OtherActor :type "Actor Object Reference"))
  (bind _returnvalue (`GameplayStatics.GetObjectClass` OtherActor))
  (bind _tostop (`self.Tostop`))
  (bind _returnvalue_2 (`KismetMathLibrary.MakeTransform` (`self.startLoc`) (struct) (0.0 0.0 0.0)))
  (if (`self.stop`)
    _
    (elif (`KismetMathLibrary.ClassIsChildOf` _returnvalue "/Game/SideScrollerCPP/Blueprints/SideScrollerCharacter2.SideScrollerCharacter2_C")
      (set `self.onHit` true)
      (elif (`KismetMathLibrary.ClassIsChildOf` _returnvalue "/Game/SideScrollerCPP/Blueprints/SideScrollerCharacter.SideScrollerCharacter_C")
        _
        (elif (`KismetMathLibrary.ClassIsChildOf` _returnvalue "BellFlowNewLB_Blueprint2_C")
          (if (not (== (`self.K2_GetActorLocation`) (`self.K2_GetActorLocation` OtherActor)))
            (set `self.stop` true)
            (set `self.hitflow` true)
            (`/Engine/EditorBlueprintResources/StandardMacros.IncrementInt` _tostop
              (:`  `
                (if (== (`self.growNum`) 0) :!label _label
                  (`|SpawnActorFromClass` "/Game/Blueprints/VineBud_Blueprint.VineBud_Blueprint_C" _returnvalue_2 "Undefined" "OverrideRootScale")
                  (else
                    (bind _returnvalue_3 (`|SpawnActorFromClass` "BellFlowNewLB_Blueprint2_C" _returnvalue_2 "Undefined" "OverrideRootScale"))
                    (set `/Game/Blueprints/BellFlowNewLB_Blueprint2.startScale` (`self.startScale`) _returnvalue_3)
                    (set `/Game/Blueprints/BellFlowNewLB_Blueprint2.growNum` (- (`self.growNum`) 1) _returnvalue_3))))))
          (elif (== (`self.Tostop`) 0)
            (set `self.onGrow` false)
            (set `self.stop` true)
            (`/Engine/EditorBlueprintResources/StandardMacros.IncrementInt` _tostop
              (:`  `
                (goto _label)))))))))

(event `self.ReceiveTick`
  (params (DeltaSeconds :type "Float (single-precision)"))
  (bind _returnvalue (`self.GetActorScale3D`))
  (bind _returnvalue_2 (`self.GetActorScale3D`))
  (bind _ctr (`self.ctr`))
  (if (`self.stop`)
    (if (< (.x _returnvalue_2) 0.75)
      (`self.K2_AddActorWorldOffset` (0.0 0.0 0.09))
      (`self.SetActorScale3D` (+ _returnvalue_2 (0.003 0.003 0.003))))
    (if (`self.hitflow`)
      _
      (elif (< _ctr 10)
        (`/Engine/EditorBlueprintResources/StandardMacros.IncrementInt` _ctr
          (:`  `
            (`|ExecutionSequence` :!label _label_2
              (:`then_0`
                (if (`self.onHit`)
                  (`self.K2_AddActorWorldOffset` (0.0 0.0 -2.0))
                  (`self.K2_AddActorWorldRotation` (struct :`Yaw` 1.0))
                  (if (< (.z (`self.K2_GetActorLocation`)) 25470.0)
                    (if (`self.stop`)
                      (bind (_direction _blend) (`Timeline|Timeline_0` :!via `Reverse` :!label _label_3)
                        (:`Update`
                          (`MeshComponent.SetScalarParameterValueOnMaterials` (`self.StaticMesh`) "Blend" _blend)))
                      (else
                        (`self.SetActorScale3D` (- (`self.GetActorScale3D`) (0.0008 0.0008 0.0008)))
                        (goto _label_3))))))
              (:`then_1`
                (if (`self.onGrow`)
                  (if (< (.x _returnvalue) (.x (`self.startScale`)))
                    (`self.SetActorScale3D` (+ _returnvalue (0.02 0.02 0.02)))
                    (else
                      (set `self.onGrow` false))))))))))
    (else
      (goto _label_2))))

(fn `UserConstructionScript`)
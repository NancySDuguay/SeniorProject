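; Flower actor that grows upward once SetWaterHit flags it as hit by water.
; Tick counts frames up to FlowerGrowHeight as a delay, then sets IsHit on every StartWater_Blueprint.
; Inside that loop it raises flower and TheStem, widening the flower and stretching the stem.
; Leaf1 gets MoveT during growth and MoveF once the flower is within the target height band above its starting Z.
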(event `self.ReceiveBeginPlay`
  (set `self.StartZ` (.z (`self.K2_GetActorLocation`))))

(event `self.ReceiveTick`
  (params (DeltaSeconds :type "Float (single-precision)"))
  (bind _thestem (`self.theStem`))
  (bind _ctr (`self.ctr`))
  (bind _flowergrowheight (`self.FlowerGrowHeight`))
  (bind _returnvalue (+ (`self.StartZ`) (`self.FlowerGrowHeight`)))
  (if (`self.WaterHit`)
    (if (`KismetMathLibrary.InRange_FloatFloat` _ctr _flowergrowheight (+ _flowergrowheight 3.0))
      (set `self.flowerGrow` true)
      (bind _outactors (`GameplayStatics.GetAllActorsOfClass` "/Game/Blueprints/StartWater_Blueprint.StartWater_Blueprint_C"))
      (for _array_element _outactors
        (set `/Game/Blueprints/StartWater_Blueprint.IsHit` true _array_element)
        (if (`KismetMathLibrary.InRange_FloatFloat` (.z (`self.K2_GetActorLocation`)) _returnvalue (+ _returnvalue 3.0))
          (set `self.flowerGrow` false)
          (`/Game/Blueprints/Leaf_Blueprint_2.Move_F` (`self.Leaf1`))
          (else
            (`/Game/Blueprints/Leaf_Blueprint_2.Move_T` (`self.Leaf1`))
            (`self.K2_AddActorWorldOffset` (`KismetMathLibrary.MakeVector` 0.0 0.0 2.0))
            (`self.SetActorScale3D` (+ (`self.GetActorScale3D`) (0.005 0.005 0.0)))
            (`self.K2_AddActorWorldOffset` _thestem (0.0 0.0 2.0) false false)
            (`self.SetActorScale3D` _thestem (+ (`self.GetActorScale3D` _thestem) (0.0 0.0 2.5))))))
      (else
        (set `self.Ctr` (`KismetMathLibrary.Conv_IntToDouble` (+ (`KismetMathLibrary.FTrunc` _ctr) 1)))))))

(fn `SetWaterHit`
  (set `self.WaterHit` true))

(fn `UserConstructionScript`)
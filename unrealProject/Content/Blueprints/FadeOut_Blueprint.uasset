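; An overlap-triggered actor that fades out and swaps streamed levels, moving from Teeter_totter_2 to Water_Rising.
; On any actor overlap it prints a debug string, then searches all Matinee actors for the one named "FadeOut" and plays it.
; After a short delay it loads Water_Rising as visible without blocking, then unloads Teeter_totter_2.
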(event `self.ReceiveActorBeginOverlap`
  (params (OtherActor :type "Actor Object Reference"))
  (`KismetSystemLibrary.PrintString` "FADE")
  (bind _outactors (`GameplayStatics.GetAllActorsOfClass` "/Script/Engine.MatineeActor"))
  (for _array_element _outactors
    (if (`KismetStringLibrary.EqualEqual_StrStr` (`KismetSystemLibrary.GetObjectName` _array_element) "FadeOut")
      (`MatineeActor.Play` _array_element)
      (`KismetSystemLibrary.Delay` 1.0)
      (`GameplayStatics.LoadStreamLevel` "Water_Rising" true)
      (`GameplayStatics.UnloadStreamLevel` "Teeter_totter_2"))))

(fn `UserConstructionScript`)
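; VineCollider is a trigger actor that marks when either of the two players stands at a vine in a side-scroller.
; On begin overlap it sets CanClimb on player 1's SideScrollerCharacter2 and IsInFrontOfBranch on player 0's SideScrollerCharacter.
; End overlap clears the same flags.
; Each player is identified by comparing the overlapping actor to the pawn at that index, then cast to its character class.
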(event `self.ReceiveActorBeginOverlap`
  (params (OtherActor :type "Actor Object Reference"))
  (bind _returnvalue (`GameplayStatics.GetPlayerPawn` 0))
  (`|ExecutionSequence`
    (:`then_0`
      (if (== OtherActor (`GameplayStatics.GetPlayerPawn` 1))
        (bind _asside_scroller_character_2 (cast `/Game/SideScrollerCPP/Blueprints/SideScrollerCharacter2` (`GameplayStatics.GetPlayerCharacter` 1)))
        (set `/Game/SideScrollerCPP/Blueprints/SideScrollerCharacter2.canClimb` true _asside_scroller_character_2)))
    (:`then_1`
      (if (== OtherActor _returnvalue)
        (bind _asside_scroller_character (cast `/Game/SideScrollerCPP/Blueprints/SideScrollerCharacter` _returnvalue))
        (set `/Game/SideScrollerCPP/Blueprints/SideScrollerCharacter.isInFrontOfBranch` true _asside_scroller_character)))))

(event `self.ReceiveActorEndOverlap`
  (params (OtherActor :type "Actor Object Reference"))
  (bind _returnvalue (`GameplayStatics.GetPlayerPawn` 0))
  (`|ExecutionSequence`
    (:`then_0`
      (if (== OtherActor (`GameplayStatics.GetPlayerPawn` 1))
        (bind _asside_scroller_character_2 (cast `/Game/SideScrollerCPP/Blueprints/SideScrollerCharacter2` (`GameplayStatics.GetPlayerCharacter` 1)))
        (set `/Game/SideScrollerCPP/Blueprints/SideScrollerCharacter2.canClimb` false _asside_scroller_character_2)))
    (:`then_1`
      (if (== OtherActor _returnvalue)
        (bind _asside_scroller_character (cast `/Game/SideScrollerCPP/Blueprints/SideScrollerCharacter` _returnvalue))
        (set `/Game/SideScrollerCPP/Blueprints/SideScrollerCharacter.isInFrontOfBranch` false _asside_scroller_character)))))

(fn `UserConstructionScript`)
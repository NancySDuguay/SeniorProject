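; Cut boulder piece, with berry/fruit naming, that plays a glow effect and can move together with a paired piece.
; Tick triggers a FlipFlop-driven timeline on the material's Blend when visibility changes or IsGlowSmall is set, suspending physics and collision until finished.
; WhichBerry marks the main piece, which rises by per-tick counters, while the other steps toward OtherFruit axis by axis.
; The proximity outline function Highlight is never run.
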(event `CustomEvent`)

(event `self.ReceiveBeginPlay`
  (bind _staticmeshcomponent (`self.StaticMeshComponent`))
  ;[1 1 1] Set start position and create instance material that will change later
  (`PrimitiveComponent.CreateDynamicMaterialInstance` _staticmeshcomponent 0 (`PrimitiveComponent.GetMaterial` _staticmeshcomponent 0)))

(event `self.ReceiveTick`
  (params (DeltaSeconds :type "Float (single-precision)"))
  (bind _staticmeshcomponent (`self.StaticMeshComponent`))
  (bind _ctrmoveup (`self.ctrMoveUp`))
  (`|ExecutionSequence`
    (:`then_0`
      ;[1 1 1] Hasn't finished glowing
      (if (not (`self.finishedGlow`))
        (`PrimitiveComponent.SetSimulatePhysics` (`self.StaticMeshComponent`) false)
        (`self.SetActorEnableCollision` false)))
    (:`then_1`
      (if (`SceneComponent.IsVisible` _staticmeshcomponent)
        (`|ExecutionSequence`
          (:`then_0`
            (if (!= (`self.ctr`) 50)
              (`self.SetActorEnableCollision` false)
              (if (`self.WhichBerry`)
                (`KismetSystemLibrary.PrintString` (`KismetStringLibrary.Conv_VectorToString` (`self.K2_GetActorLocation`)))
                (`self.K2_AddActorWorldOffset` (0.0 0.0 1.2))
                (else
                  (`self.K2_AddActorWorldOffset` (0.0 0.0 0.0))))
              (`/Engine/EditorBlueprintResources/StandardMacros.IncrementInt` (`self.ctr`))))
          (:`then_1`
            (if (not (`self.calledOnce`))
              (`PrimitiveComponent.SetSimulatePhysics` _staticmeshcomponent false)
              (set `self.calledOnce` true)
              (bind _isa (`/Engine/EditorBlueprintResources/StandardMacros.FlipFlop` :!label _label)
                (:`A`
                  (bind (_direction _blend) (`Timeline|Timeline_1` :!via `ReverseFromEnd` :!label _label_2)
                    (:`Update`
                      (`self.SetActorEnableCollision` false)
                      (`MeshComponent.SetScalarParameterValueOnMaterials` (`self.StaticMeshComponent`) "Blend" _blend))
                    (:`Finished`
                      (`self.SetActorEnableCollision` true)
                      (`PrimitiveComponent.SetSimulatePhysics` (`self.StaticMeshComponent`) true)
                      (set `self.finishedGlow` true)
                      (set `self.ctrMoveUp` 0)
                      (if (not _isa)
                        (set `self.calledOnce` false)
                        (set `self.ctr` 0)
                        (set `self.moveTogether` false)))))
                (:`B`
                  (goto _label_2 :!via `PlayFromStart`))))))
        (else
          (`self.K2_SetActorRotation` (struct))
          (if (`self.calledOnce`)
            (set `self.calledOnce` false)
            (goto _label)))))
    (:`then_2`
      (`|ExecutionSequence`
        (:`then_0`
          (if (`self.IsGlowSmall`)
            (`PrimitiveComponent.SetSimulatePhysics` _staticmeshcomponent false)
            (`self.SetActorEnableCollision` false)
            (set `self.moveTogether` true)
            (set `self.IsGlowSmall` false)
            (goto _label)))
        (:`then_1`
          (if (`self.moveTogether`)
            ;[1 1 1] If it's not the main berry, move it constantly until it's in the other berry's position
            (if (not (`self.WhichBerry`))
              (`|ExecutionSequence`
                (:`then_0`
                  (`/Engine/EditorBlueprintResources/StandardMacros.CompareFloat` (.x (`self.K2_GetActorLocation`)) (.x (`self.K2_GetActorLocation` (`self.OtherFruit`)))
                    (:`>`
                      (`self.K2_AddActorWorldOffset` (-0.75 0.0 0.0)))
                    (:`<`
                      (`self.K2_AddActorWorldOffset` (0.75 0.0 0.0)))))
                (:`then_1`
                  (`/Engine/EditorBlueprintResources/StandardMacros.CompareFloat` (.y (`self.K2_GetActorLocation`)) (.y (`self.K2_GetActorLocation` (`self.OtherFruit`)))
                    (:`>`
                      (`self.K2_AddActorWorldOffset` (0.0 -0.75 0.0)))
                    (:`<`
                      (`self.K2_AddActorWorldOffset` (0.0 0.75 0.0)))))
                (:`then_2`
                  (`/Engine/EditorBlueprintResources/StandardMacros.CompareFloat` (.z (`self.K2_GetActorLocation`)) (.z (`self.K2_GetActorLocation` (`self.OtherFruit`)))
                    (:`>`
                      (`self.K2_AddActorWorldOffset` (0.0 0.0 -0.75)))
                    (:`<`
                      (`self.K2_AddActorWorldOffset` (0.0 0.0 0.75))))))
              (else
                (`/Engine/EditorBlueprintResources/StandardMacros.CompareInt` _ctrmoveup 60
                  (:`<`
                    (`self.K2_AddActorWorldOffset` (0.0 0.0 0.5))
                    (`/Engine/EditorBlueprintResources/StandardMacros.IncrementInt` _ctrmoveup)))))))))))

(fn `Highlight`
  (if (<= (`KismetMathLibrary.VSize` (- (`self.K2_GetActorLocation` (`GameplayStatics.GetPlayerPawn` 1)) (`self.K2_GetActorLocation`))) 150.0)
    (`PrimitiveComponent.SetRenderCustomDepth` (`self.StaticMeshComponent`) true)
    (else
      (`PrimitiveComponent.SetRenderCustomDepth` (`self.StaticMeshComponent`) false))))

(fn `UserConstructionScript`)
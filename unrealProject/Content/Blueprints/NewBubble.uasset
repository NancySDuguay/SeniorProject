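; A rising bubble actor that bursts when SideScrollerCharacter2 touches it or Char2 comes within range.
; Each tick it grows from a small scale to full size, then drifts upward until destroyed above a height limit.
; Passing an exact Z height spawns a replacement at the start point, handing on Char2.
; Bursting disables collision, hides the mesh and plays a particle effect, but the hidden actor keeps rising to continue the cycle.
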(event `self.ReceiveActorBeginOverlap`
  (params (OtherActor :type "Actor Object Reference"))
  (if (`KismetMathLibrary.ClassIsChildOf` (`GameplayStatics.GetObjectClass` OtherActor) "/Game/SideScrollerCPP/Blueprints/SideScrollerCharacter2.SideScrollerCharacter2_C") :!label _label
    (`self.SetActorEnableCollision` false :!label _label_2)
    (if (not (`self.beenHit`))
      (`SceneComponent.SetVisibility` (`self.StaticMesh`) false false)
      (`GameplayStatics.SpawnEmitterAtLocation` "/Game/ParticleSystem/Sprite/P_BubbleBurst.P_BubbleBurst" (+ (`self.K2_GetActorLocation`) (0.0 0.0 50.0)))
      (set `self.beenHit` true))))

(event `self.ReceiveHit`
  (params (MyComp :type "PrimitiveComponent Object Reference") (Other :type "Actor Object Reference") (OtherComp :type "PrimitiveComponent Object Reference") (bSelfMoved :type Boolean) (HitLocation :type "Vector Structure") (HitNormal :type "Vector Structure") (NormalImpulse :type "Vector Structure") (Hit :type "HitResult Structure (by ref)"))
  (goto _label))

(event `self.ReceiveBeginPlay`
  (`self.SetActorScale3D` (0.1 0.1 0.1))
  (set `self.startLoc` (`self.K2_GetActorLocation`)))

(event `self.ReceiveTick`
  (params (DeltaSeconds :type "Float (single-precision)"))
  (bind _returnvalue (`self.GetActorScale3D`))
  (`|ExecutionSequence`
    (:`then_0`
      (if (`KismetMathLibrary.InRange_FloatFloat` (.x _returnvalue) 1.0 1.1)
        (`self.K2_AddActorWorldOffset` (0.0 0.0 2.0))
        (if (== (.z (`self.K2_GetActorLocation`)) 11320.0)
          (bind _returnvalue_2 (`|SpawnActorFromClass` "NewBubble_C" (`KismetMathLibrary.MakeTransform` (`self.startLoc`) (struct) (0.1 0.1 0.1)) "Undefined" "OverrideRootScale"))
          (set `/Game/Blueprints/NewBubble.char2` (`self.char2`) _returnvalue_2)
          (elif (> (.z (`self.K2_GetActorLocation`)) 12200.0)
            (`self.K2_DestroyActor`)))
        (else
          (`self.SetActorScale3D` (+ _returnvalue (0.005 0.005 0.005))))))
    (:`then_1`
      (if (and (`KismetMathLibrary.InRange_FloatFloat` (- (.x (`self.K2_GetActorLocation` (`self.char2`))) (.x (`self.K2_GetActorLocation`))) -100.0 100.0) (and (`KismetMathLibrary.InRange_FloatFloat` (- (.y (`self.K2_GetActorLocation` (`self.char2`))) (.y (`self.K2_GetActorLocation`))) -100.0 100.0) (`KismetMathLibrary.InRange_FloatFloat` (- (.z (`self.K2_GetActorLocation` (`self.char2`))) (.z (`self.K2_GetActorLocation`))) 0.0 200.0)))
        (goto _label_2)))))

(fn `UserConstructionScript`)
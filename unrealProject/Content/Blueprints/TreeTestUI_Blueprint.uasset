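; Test actor that shows a TreeWidget on screen and drives it from the actor's height in the world.
; On BeginPlay it creates the widget and adds it to the viewport.
; Each Tick, UpdatePositionUI rescales world Z against a hardcoded offset and range.
; When that value differs from the one stored in the Position progress-bar struct, it saves it, prints it for debugging and passes it to the widget's UpdatePos.
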(event `self.ReceiveBeginPlay`
  (bind _returnvalue (`|CreateWidget` "/Game/UI/TreeProgressionUI/TreeWidget.TreeWidget_C"))
  (bind _output_get (set `self.treeWidget` _returnvalue))
  (`UserWidget.AddToViewport` _output_get 0))

(event `self.ReceiveTick`
  (params (DeltaSeconds :type "Float (single-precision)"))
  (`self.UpdatePositionUI`))

(fn `UpdatePositionUI`
  (bind (_position_max _position_current _position_desired) (break `/Game/UI/TreeProgressionUI/ProgressBarVars` (`self.position`)))
  (bind _returnvalue (/ (- (.z (`self.K2_GetActorLocation`)) 17400.0) 1100.0))
  (if (!= _returnvalue _position_desired)
    (`|ExecutionSequence`
      (:`then_0`
        (bind _output_get (set `self.position` (make `/Game/UI/TreeProgressionUI/ProgressBarVars` 0.0 0.0 _returnvalue)))
        (`KismetSystemLibrary.PrintString` (`KismetStringLibrary.Conv_DoubleToString` (`.Desired_6_DE4A4AE8462D1A3336A02EB21A90DC78` (break `/Game/UI/TreeProgressionUI/ProgressBarVars` _output_get)))))
      (:`then_1`
        (`/Game/UI/TreeProgressionUI/TreeWidget.updatePos` (`self.treeWidget`) _returnvalue)))))

(fn `UserConstructionScript`)
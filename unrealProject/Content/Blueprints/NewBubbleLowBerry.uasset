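; NewBubbleLowBerry is a self-respawning bubble that grows from a small scale, then rises until it bursts at a fixed height.
; Tick drives growth and movement, spawning a replacement at the start location just below that height, then destroying itself.
; SideScrollerCharacter2 overlap or a per-tick proximity check on player index 1 pops it once with particles and sound.
; Popped or BoulderB-hit bubbles are only hidden with collision disabled, so the respawn cycle continues.
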(event `self.ReceiveHit`
  (params (MyComp :type "PrimitiveComponent Object Reference") (Other :type "Actor Object Reference") (OtherComp :type "PrimitiveComponent Object Reference") (bSelfMoved :type Boolean) (HitLocation :type "Vector Structure") (HitNormal :type "Vector Structure") (NormalImpulse :type "Vector Structure") (Hit :type "HitResult Structure (by ref)"))
  (if (`KismetMathLibrary.ClassIsChildOf` (`GameplayStatics.GetObjectClass` Other) "/Game/Blueprints/BoulderB.BoulderB_C")
    (`self.SetActorEnableCollision` false)
    (`SceneComponent.SetVisibility` (`self.StaticMesh`) false false)))

(event `self.ReceiveActorBeginOverlap`
  (params (OtherActor :type "Actor Object Reference"))
  (if (`KismetMathLibrary.ClassIsChildOf` (`GameplayStatics.GetObjectClass` OtherActor) "/Game/SideScrollerCPP/Blueprints/SideScrollerCharacter2.SideScrollerCharacter2_C")
    (`KismetSystemLibrary.PrintString` "Overlap")
    (`self.SetActorEnableCollision` false :!label _label)
    (if (not (`self.beenHit`))
      (`SceneComponent.SetVisibility` (`self.StaticMesh`) false false)
      (`GameplayStatics.SpawnEmitterAtLocation` "/Game/ParticleSystem/Sprite/P_BubbleBurst.P_BubbleBurst" (+ (`self.K2_GetActorLocation`) (0.0 0.0 50.0)))
      (`GameplayStatics.PlaySoundAtLocation` "/Game/MusicSound/BubblePop.BubblePop")
      (set `self.beenHit` true))))

(event `self.ReceiveBeginPlay`
  (`self.SetActorScale3D` (0.1 0.1 0.1))
  (set `self.startLoc` (`self.K2_GetActorLocation`)))

(event `self.ReceiveTick`
  (params (DeltaSeconds :type "Float (single-precision)"))
  (bind _returnvalue (`self.GetActorScale3D`))
  (`|ExecutionSequence`
    (:`then_0`
      (if (`KismetMathLibrary.InRange_FloatFloat` (.x _returnvalue) 1.0 1.1)
        (`self.K2_AddActorWorldOffset` (0.0 0.0 2.0))
        (if (== (.z (`self.K2_GetActorLocation`)) 25480.0)
          (`|SpawnActorFromClass` "NewBubbleLowBerry_C" (`KismetMathLibrary.MakeTransform` (`self.startLoc`) (struct) (0.1 0.1 0.1)) "Undefined" "OverrideRootScale")
          (elif (> (.z (`self.K2_GetActorLocation`)) 25490.0)
            (if (`SceneComponent.IsVisible` (`self.StaticMesh`))
              (`GameplayStatics.SpawnEmitterAtLocation` "/Game/ParticleSystem/Sprite/P_BubbleBurst.P_BubbleBurst" (+ (`self.K2_GetActorLocation`) (0.0 0.0 50.0)))
              (`GameplayStatics.PlaySoundAtLocation` "/Game/MusicSound/BubblePop.BubblePop"))
            (`self.K2_DestroyActor`)))
        (else
          (`self.SetActorScale3D` (+ _returnvalue (0.005 0.005 0.005))))))
    (:`then_1`
      (if (and (`KismetMathLibrary.InRange_FloatFloat` (- (.x (`self.K2_GetActorLocation` (`GameplayStatics.GetPlayerCharacter` 1))) (.x (`self.K2_GetActorLocation`))) -100.0 100.0) (and (`KismetMathLibrary.InRange_FloatFloat` (- (.y (`self.K2_GetActorLocation` (`GameplayStatics.GetPlayerCharacter` 1))) (.y (`self.K2_GetActorLocation`))) -100.0 100.0) (`KismetMathLibrary.InRange_FloatFloat` (- (.z (`self.K2_GetActorLocation` (`GameplayStatics.GetPlayerCharacter` 1))) (.z (`self.K2_GetActorLocation`))) 0.0 200.0)))
        (goto _label)))))

(fn `UserConstructionScript`)
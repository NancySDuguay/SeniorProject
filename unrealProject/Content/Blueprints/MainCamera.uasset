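; Main camera actor for a two-player game that frames both player pawns as they move.
; Each tick it derives the camera component's relative Y and Z from the players' midpoint and the actor's location, adding a height offset.
; When the players' Y separation exceeds a fixed threshold, the excess becomes a negative X offset that zooms out by moving the camera rather than changing field of view.
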(event EventBeginPlay)

(event EventTick
  (params (DeltaSeconds :type Float%20%28single-precision%29))
  (bind _returnvalue (Transformation|GetActorLocation))
  (bind _returnvalue_2 (Game|Player|GetPlayerPawn 1))
  (bind _returnvalue_3 (Game|Player|GetPlayerPawn 0))
  (bind _returnvalue_4 (Transformation|GetActorLocation _returnvalue_2))
  (bind (_x _y _z) (Math|Vector|BreakVector _returnvalue))
  (bind _returnvalue_5 (Transformation|GetActorLocation _returnvalue_3))
  (bind (_x_2 _y_2 _z_2) (Math|Vector|BreakVector _returnvalue_5))
  (bind (_x_3 _y_3 _z_3) (Math|Vector|BreakVector _returnvalue_4))
  (bind _returnvalue_6 (- _y_2 _y_3))
  (bind _returnvalue_7 (Math|Float|Absolute(Float) _returnvalue_6))
  ;[1 1 1] Move camera based on both player's locations
  (Utilities|FlowControl|Sequence
    (:then_0
      (if (> _returnvalue_7 2e+03)
        (Variables|Default|SetxZoom (* (- _returnvalue_7 2e+03) -1.0))
        (else
          (Variables|Default|SetxZoom 0.0))))
    (:then_1
      (bind _output_get (Variables|Default|SetnewLocation (Math|Vector|MakeVector (Variables|Default|GetxZoom) (|(a-b) _y (|((a+b)/2) _y_2 _y_3)) (|(a-b) (Variables|Default|GetzOffset) (|(a-b) _z (|((a+b)/2) _z_2 _z_3))))))
      (Transformation|SetRelativeLocation (Variables|CameraActor|GetCameraComponent) _output_get false false))))

(fn ConstructionScript)
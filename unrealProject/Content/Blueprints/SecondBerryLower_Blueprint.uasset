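; A side-scroller flower bud/berry platform that sinks while the player character (Mai) stands on it and rises back when she leaves.
; Overlap events track Mai and stop lowering on ground contact, while Tick compares the bud's Z to hard-coded world heights to set lower/rise flags.
; Per-tick fixed offsets move the bud and tilt and shift a referenced Branch actor with it.
; Tick also enables overlap events on the last MergedVine found, if visible.
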(event `self.ReceiveActorEndOverlap`
  (params (OtherActor :type "Actor Object Reference"))
  ;[1 1 1] Mai overlap
  (if (`KismetMathLibrary.ClassIsChildOf` (`GameplayStatics.GetObjectClass` OtherActor) "/Game/SideScrollerCPP/Blueprints/SideScrollerCharacter2.SideScrollerCharacter2_C")
    (set `self.berryMaiOverlap` false)))

(event `self.ReceiveActorBeginOverlap`
  (params (OtherActor :type "Actor Object Reference"))
  (bind _returnvalue (`GameplayStatics.GetObjectClass` OtherActor))
  ;[1 1 1] Mai overlap
  (if (`KismetMathLibrary.ClassIsChildOf` _returnvalue "/Game/Blueprints/vine_full.vine_full_C")
    _
    (elif (`KismetMathLibrary.ClassIsChildOf` _returnvalue "/Game/Blueprints/Ground_Blueprint.Ground_Blueprint_C")
      (set `self.LowerBerry` false)
      (elif (`KismetMathLibrary.ClassIsChildOf` _returnvalue "/Game/SideScrollerCPP/Blueprints/SideScrollerCharacter2.SideScrollerCharacter2_C")
        (set `self.berryMaiOverlap` true)))))

(event `self.ReceiveTick`
  (params (DeltaSeconds :type "Float (single-precision)"))
  (`|ExecutionSequence`
    (:`then_0`
      ;[1 1 1] Check if Mai is on Flower Bud, set lowering & raising
      (if (`self.berryMaiOverlap`)
        (if (`KismetMathLibrary.InRange_FloatFloat` (.z (`self.K2_GetActorLocation`)) 15884.0 15886.0)
          (if (`self.berryMaiOverlap`)
            (set `self.LowerBerry` true)
            (set `self.RiseBerry` false)
            (else
              (set `self.LowerBerry` false)
              (set `self.RiseBerry` false)))
          (elif (`KismetMathLibrary.InRange_FloatFloat` (.z (`self.K2_GetActorLocation`)) 15744.0 15746.0)
            (set `self.LowerBerry` false)))
        (elif (`KismetMathLibrary.InRange_FloatFloat` (.z (`self.K2_GetActorLocation`)) 15744.0 15746.0)
          (set `self.RiseBerry` true)
          (elif (`KismetMathLibrary.InRange_FloatFloat` (.z (`self.K2_GetActorLocation`)) 15884.0 15886.0)
            (set `self.RiseBerry` false)
            (elif (`KismetMathLibrary.InRange_FloatFloat` (.z (`self.K2_GetActorLocation`)) 15744.0 15746.0)
              (set `self.RiseBerry` true))))))
    (:`then_1`
      ;[1 1 1] Lowering Bud & Branch
      (if (`self.berryMaiOverlap`)
        (if (`self.LowerBerry`)
          (`self.K2_AddActorWorldOffset` (`KismetMathLibrary.MakeVector` 0.0 0.0 -2.0))
          (`self.K2_AddActorWorldRotation` (`self.Branch`) (`KismetMathLibrary.MakeRotator` 0.035 0.0) false false)
          (`self.K2_AddActorWorldOffset` (`self.Branch`) (`KismetMathLibrary.MakeVector` 0.0 0.3) false false))))
    (:`then_2`
      ;[1 1 1] Rising Bud & Branch
      (if (`self.berryMaiOverlap`)
        _
        (elif (`self.RiseBerry`)
          (`self.K2_AddActorWorldOffset` (`KismetMathLibrary.MakeVector` 0.0 0.0 2.0))
          (`self.K2_AddActorWorldRotation` (`self.Branch`) (`KismetMathLibrary.MakeRotator` -0.035 0.0) false false)
          (`self.K2_AddActorWorldOffset` (`self.Branch`) (`KismetMathLibrary.MakeVector` 0.0 -0.3) false false))))
    (:`then_3`
      ;[1 1 1] If Mai gets off Bud, Rise Bud & Branch
      (if (`self.berryMaiOverlap`)
        _
        (elif (`KismetMathLibrary.InRange_FloatFloat` (.z (`self.K2_GetActorLocation`)) 0.0 15884.0)
          (`self.K2_AddActorWorldOffset` (`KismetMathLibrary.MakeVector` 0.0 0.0 2.0))
          (`self.K2_AddActorWorldRotation` (`self.Branch`) (`KismetMathLibrary.MakeRotator` -0.035 0.0) false false)
          (`self.K2_AddActorWorldOffset` (`self.Branch`) (`KismetMathLibrary.MakeVector` 0.0 -0.3) false false))))
    (:`then_4`
      (bind _outactors (`GameplayStatics.GetAllActorsOfClass` "/Game/mergedVine.mergedVine_C"))
      (for _array_element _outactors
        _)
      (bind _staticmeshcomponent (`StaticMeshActor.StaticMeshComponent` _array_element))
      (if (`SceneComponent.IsVisible` _staticmeshcomponent)
        (set `PrimitiveComponent.bGenerateOverlapEvents` true _staticmeshcomponent)))))

(fn `UserConstructionScript`)
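; Boulder actor whose material glows through a timeline-driven "Blend" parameter and which can be outlined when a player is near.
; Tick starts the glow once when IsGlow is set, then a FlipFlop reverses it and physics simulation is switched off.
; Hiding the mesh clears the one-shot flag and triggers the FlipFlop again.
; A separate Highlight function toggles custom depth by distance to player pawn index 1.
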(event `self.ReceiveHit`
  (params (MyComp :type "PrimitiveComponent Object Reference") (Other :type "Actor Object Reference") (OtherComp :type "PrimitiveComponent Object Reference") (bSelfMoved :type Boolean) (HitLocation :type "Vector Structure") (HitNormal :type "Vector Structure") (NormalImpulse :type "Vector Structure") (Hit :type "HitResult Structure (by ref)")))

(event `self.ReceiveBeginPlay`
  (bind _staticmeshcomponent (`self.StaticMeshComponent`))
  (`PrimitiveComponent.CreateDynamicMaterialInstance` _staticmeshcomponent 0 (`PrimitiveComponent.GetMaterial` _staticmeshcomponent 0)))

(event `self.ReceiveTick`
  (params (DeltaSeconds :type "Float (single-precision)"))
  (bind _staticmeshcomponent (`self.StaticMeshComponent`))
  (`|ExecutionSequence`
    (:`then_0`
      (if (`self.IsGlow`)
        (if (not (`self.calledOnce`))
          (set `self.calledOnce` true)
          (bind _isa (`/Engine/EditorBlueprintResources/StandardMacros.FlipFlop` :!label _label)
            (:`A`
              (bind (_direction _blend) (`Timeline|Timeline_0` :!via `PlayFromStart` :!label _label_2)
                (:`Update`
                  (`MeshComponent.SetScalarParameterValueOnMaterials` (`self.StaticMeshComponent`) "Blend" _blend))
                (:`Finished`
                  (set `self.IsGlow` false)
                  (if _isa
                    (set `self.doneGlow` true)))))
            (:`B`
              (goto _label_2 :!via `ReverseFromEnd`))))))
    (:`then_1`
      (if (`SceneComponent.IsVisible` _staticmeshcomponent)
        (if (`self.doneGlow`)
          (`PrimitiveComponent.SetSimulatePhysics` _staticmeshcomponent false)
          (set `self.doneGlow` false)
          (goto _label))
        (elif (`self.calledOnce`)
          (set `self.calledOnce` false)
          (goto _label))))))

(fn `Highlight`
  (if (<= (`KismetMathLibrary.VSize` (- (`self.K2_GetActorLocation` (`GameplayStatics.GetPlayerPawn` 1)) (`self.K2_GetActorLocation`))) 150.0)
    (`PrimitiveComponent.SetRenderCustomDepth` (`self.StaticMeshComponent`) true)
    (else
      (`PrimitiveComponent.SetRenderCustomDepth` (`self.StaticMeshComponent`) false))))

(fn `UserConstructionScript`)
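; ChangeAngle is an overlap-triggered actor that changes the plane along which boulders can move.
; On overlap it prints "Hit" and checks whether the other actor derives from CutBoulderB or BoulderB.
; For either class, it switches that actor's static mesh components to an XZ-plane constraint mode.
; The disconnected plane-constraint and character-movement nodes never run.
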(event `self.ReceiveTick`
  (params (DeltaSeconds :type "Float (single-precision)")))

(event `self.ReceiveActorBeginOverlap`
  (params (OtherActor :type "Actor Object Reference"))
  (bind _returnvalue (`GameplayStatics.GetObjectClass` OtherActor))
  (`KismetSystemLibrary.PrintString` "Hit")
  (if (`KismetMathLibrary.ClassIsChildOf` _returnvalue "/Game/Blueprints/cutBoulderB.cutBoulderB_C")
    (`PrimitiveComponent.SetConstraintMode` (`self.K2_GetComponentsByClass` OtherActor "/Script/Engine.StaticMeshComponent") "XZPlane" :!label _label)
    (elif (`KismetMathLibrary.ClassIsChildOf` _returnvalue "/Game/Blueprints/BoulderB.BoulderB_C")
      (goto _label))))

(event `self.ReceiveHit`
  (params (MyComp :type "PrimitiveComponent Object Reference") (Other :type "Actor Object Reference") (OtherComp :type "PrimitiveComponent Object Reference") (bSelfMoved :type Boolean) (HitLocation :type "Vector Structure") (HitNormal :type "Vector Structure") (NormalImpulse :type "Vector Structure") (Hit :type "HitResult Structure (by ref)")))

(fn `UserConstructionScript`)
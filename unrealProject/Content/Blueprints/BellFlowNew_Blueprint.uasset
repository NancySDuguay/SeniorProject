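; Bell flower actor that falls and spins when SideScrollerCharacter2 touches it, then regrows at its original spot.
; Hit and overlap events set flags that Tick uses to move, grow or shrink it, with a timeline blending its material below a height threshold.
; Touching other non-character, non-bellflower actors makes it shrink, sink and destroy itself.
; Only the overlap path spawns the zero-scale replacement, which inherits the original scale as its growth target.
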(event `self.ReceiveBeginPlay`
  (bind _staticmesh (`self.StaticMesh`))
  (`|ExecutionSequence`
    (:`then_0`
      (set `self.startLoc` (`self.K2_GetActorLocation`))
      (set `self.onGrow` true)
      (set `self.onHit` false)
      (set `self.startScale` (`self.GetActorScale3D`)))
    (:`then_1`
      (`PrimitiveComponent.CreateDynamicMaterialInstance` _staticmesh 0 (`PrimitiveComponent.GetMaterial` _staticmesh 0)))))

(event `self.ReceiveHit`
  (params (MyComp :type "PrimitiveComponent Object Reference") (Other :type "Actor Object Reference") (OtherComp :type "PrimitiveComponent Object Reference") (bSelfMoved :type Boolean) (HitLocation :type "Vector Structure") (HitNormal :type "Vector Structure") (NormalImpulse :type "Vector Structure") (Hit :type "HitResult Structure (by ref)"))
  (bind _returnvalue (`GameplayStatics.GetObjectClass` Other))
  (if (`KismetMathLibrary.ClassIsChildOf` _returnvalue "/Game/SideScrollerCPP/Blueprints/SideScrollerCharacter2.SideScrollerCharacter2_C")
    (set `self.onHit` true)
    (if (== (.z (`self.startLoc`)) (.z (`self.K2_GetActorLocation`)))
      (`GameplayStatics.PlaySoundAtLocation` "/Game/MusicSound/BellFlowerFallOff.BellFlowerFallOff"))
    (elif (`KismetMathLibrary.ClassIsChildOf` _returnvalue "/Game/SideScrollerCPP/Blueprints/SideScrollerCharacter.SideScrollerCharacter_C")
      _
      (elif (not (`KismetMathLibrary.ClassIsChildOf` _returnvalue "BellFlowNew_Blueprint_C"))
        (set `self.onGrow` false)
        (set `self.onHit` false)
        (`KismetSystemLibrary.PrintString` "1")
        (`KismetSystemLibrary.PrintString` "2")
        (set `self.desaturate` true)))))

(event `self.ReceiveActorBeginOverlap`
  (params (OtherActor :type "Actor Object Reference"))
  (bind _returnvalue (`GameplayStatics.GetObjectClass` OtherActor))
  (if (`KismetMathLibrary.ClassIsChildOf` _returnvalue "/Game/SideScrollerCPP/Blueprints/SideScrollerCharacter2.SideScrollerCharacter2_C")
    (set `self.onHit` true)
    (elif (`KismetMathLibrary.ClassIsChildOf` _returnvalue "/Game/SideScrollerCPP/Blueprints/SideScrollerCharacter.SideScrollerCharacter_C")
      _
      (elif (not (`KismetMathLibrary.ClassIsChildOf` _returnvalue "BellFlowNew_Blueprint_C"))
        (set `self.onGrow` false)
        (set `self.onHit` false)
        (if (not (`self.desaturate`))
          (`KismetSystemLibrary.PrintString` "spqwn")
          (bind _returnvalue_2 (`|SpawnActorFromClass` "BellFlowNew_Blueprint_C" (`KismetMathLibrary.MakeTransform` (`self.startLoc`) (struct) (0.0 0.0 0.0)) "Undefined" "OverrideRootScale"))
          (set `/Game/Blueprints/BellFlowNew_Blueprint.startScale` (`self.startScale`) _returnvalue_2)
          (`KismetSystemLibrary.PrintString` "2")
          (set `self.desaturate` true))))))

(event `self.ReceiveTick`
  (params (DeltaSeconds :type "Float (single-precision)"))
  (bind _returnvalue (`self.GetActorScale3D`))
  (`|ExecutionSequence`
    (:`then_0`
      (if (`self.onHit`)
        (`self.K2_AddActorWorldOffset` (0.0 0.0 -1.0))
        (`self.K2_AddActorWorldRotation` (struct :`Yaw` 1.0))
        (if (< (.z (`self.K2_GetActorLocation`)) 10800.0)
          (bind (_direction _blend) (`Timeline|Timeline_0`)
            (:`Update`
              (`MeshComponent.SetScalarParameterValueOnMaterials` (`self.StaticMesh`) "Blend" _blend))))))
    (:`then_1`
      (if (`self.onGrow`)
        (if (< (.x _returnvalue) (.x (`self.startScale`)))
          (`self.SetActorScale3D` (+ _returnvalue (0.02 0.02 0.02)))
          (else
            (set `self.onGrow` false)))))
    (:`then_2`
      (if (`self.desaturate`)
        (`self.SetActorScale3D` (- _returnvalue (0.004 0.004 0.004)))
        (`self.K2_AddActorWorldOffset` (0.0 0.0 -0.5))
        (if (<= (.x _returnvalue) 0.0)
          (`self.K2_DestroyActor`))))))

(fn `UserConstructionScript`)
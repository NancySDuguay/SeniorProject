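; Leaf actor Blueprint that moves straight up a small fixed step each tick while its IsMove flag is set.
; The MoveT and MoveF functions switch that flag on and off.
; WhichLeaf picks an immediate rise, otherwise a frame counter delays movement, so timing and speed depend on frame rate.
; An unconnected branch that would add a box component near a given Y position never runs.
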(event `self.ReceiveBeginPlay`)

(event `self.ReceiveTick`
  (params (DeltaSeconds :type "Float (single-precision)"))
  (bind _ctrleaf2 (`self.CtrLeaf2`))
  (if (`self.IsMove`)
    (if (`self.whichLeaf`)
      (`self.K2_AddActorWorldOffset` (0.0 0.0 2.0) :!label _label)
      (elif (> _ctrleaf2 220)
        (goto _label)
        (else
          (bind _result (`/Engine/EditorBlueprintResources/StandardMacros.IncrementInt` _ctrleaf2)
            (:`  `
              (`/Engine/EditorBlueprintResources/StandardMacros.IncrementInt` _result))))))))

(fn `Move_F`
  (set `self.IsMove` false))

(fn `Move_T`
  (set `self.IsMove` true))

(fn `UserConstructionScript`)
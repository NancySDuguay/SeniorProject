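; Floatable log actor that gradually levels its roll once it has entered water.
; Overlapping any PhysicsVolume-derived actor sets InWater, which is never cleared in this graph.
; While InWater, Tick interpolates the static mesh's world rotation toward its negated roll, easing it toward zero outside a small dead zone while preserving pitch and yaw.
; The graph itself applies no buoyancy force.
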(event `self.ReceiveTick`
  (params (DeltaSeconds :type "Float (single-precision)"))
  (bind _returnvalue (`SceneComponent.K2_GetComponentRotation` (`self.StaticMeshComponent`)))
  (bind _roll (.roll _returnvalue))
  (if (`self.inWater`)
    (if (> (`KismetMathLibrary.Abs` _roll) 0.1)
      (`SceneComponent.K2_SetWorldRotation` (`self.StaticMeshComponent`) (`KismetMathLibrary.RInterpTo` _returnvalue (`KismetMathLibrary.MakeRotator` (* _roll -1.0) (.pitch _returnvalue) (.yaw _returnvalue)) DeltaSeconds 1.0) false false))))

(event `self.ReceiveActorBeginOverlap`
  (params (OtherActor :type "Actor Object Reference"))
  (if (`KismetMathLibrary.ClassIsChildOf` (`GameplayStatics.GetObjectClass` OtherActor) "/Script/Engine.PhysicsVolume")
    (set `self.inWater` true)))

(fn `UserConstructionScript`)
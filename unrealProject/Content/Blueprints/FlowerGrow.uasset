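; Flower actor that grows upward after water hits it, flagged through SetWaterHit.
; Once flagged, Tick counts frames up to about 525 as a delay, then sets FlowerGrow and raises the actor one unit per frame.
; Leaf1 and Leaf2 receive MoveT while rising and MoveF once the actor reaches a hardcoded world Z band near 18000.
; Growth speed and delay depend on frame rate.
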(event `self.ReceiveTick`
  (params (DeltaSeconds :type "Float (single-precision)"))
  (bind _ctr (`self.ctr`))
  (if (`self.WaterHit`)
    (if (`KismetMathLibrary.InRange_FloatFloat` _ctr 525.0 528.0)
      (set `self.flowerGrow` true)
      (if (`KismetMathLibrary.InRange_FloatFloat` (.z (`self.K2_GetActorLocation`)) 17990.0 18000.0)
        (`/Game/Blueprints/Leaf_Blueprint_2.Move_F` (`self.Leaf1`))
        (`/Game/Blueprints/Leaf_Blueprint_2.Move_F` (`self.Leaf2`))
        (else
          (`/Game/Blueprints/Leaf_Blueprint_2.Move_T` (`self.Leaf1`))
          (`/Game/Blueprints/Leaf_Blueprint_2.Move_T` (`self.Leaf2`))
          (`self.K2_AddActorWorldOffset` (`KismetMathLibrary.MakeVector` 0.0 0.0 1.0))))
      (else
        (set `self.Ctr` (`KismetMathLibrary.Conv_IntToDouble` (+ (`KismetMathLibrary.FTrunc` _ctr) 1)))))))

(fn `SetWaterHit`
  (set `self.WaterHit` true))

(fn `UserConstructionScript`)
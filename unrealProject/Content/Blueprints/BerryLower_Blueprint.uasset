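; Berry/flower bud that sinks under Mai's weight, bending its Branch, and rises back when released.
; Mai overlapping the bud, or climbing while on FirstVine's branch, triggers lowering until LowerHeight below start or Ground contact.
; Tick moves bud and Branch by fixed per-frame steps, not scaled by delta time.
; Tick also fetches all MergedVines, but its empty loop leaves only the last for enabling overlaps when visible.
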(event `self.ReceiveBeginPlay`
  (set `self.startZ` (.z (`self.K2_GetActorLocation`))))

(event `self.ReceiveActorEndOverlap`
  (params (OtherActor :type "Actor Object Reference"))
  ;[1 1 1] Mai overlap
  (if (`KismetMathLibrary.ClassIsChildOf` (`GameplayStatics.GetObjectClass` OtherActor) "/Game/SideScrollerCPP/Blueprints/SideScrollerCharacter2.SideScrollerCharacter2_C")
    (set `self.berryMaiOverlap` false)))

(event `self.ReceiveActorBeginOverlap`
  (params (OtherActor :type "Actor Object Reference"))
  (bind _returnvalue (`GameplayStatics.GetObjectClass` OtherActor))
  ;[1 1 1] Mai overlap
  (`|ExecutionSequence`
    (:`then_0`
      (if (`KismetMathLibrary.ClassIsChildOf` _returnvalue "/Game/Blueprints/vine_full.vine_full_C")
        _
        (elif (`KismetMathLibrary.ClassIsChildOf` _returnvalue "/Game/Blueprints/Ground_Blueprint.Ground_Blueprint_C")
          (set `self.LowerBerry` false)
          (elif (`KismetMathLibrary.ClassIsChildOf` _returnvalue "/Game/SideScrollerCPP/Blueprints/SideScrollerCharacter2.SideScrollerCharacter2_C")
            (set `self.berryMaiOverlap` true)))))
    (:`then_1`
      (if (`KismetMathLibrary.ClassIsChildOf` null (`GameplayStatics.GetObjectClass` (`self.firstVine`)))
        (`KismetSystemLibrary.PrintString` (`KismetStringLibrary.Conv_BoolToString` (stale _output_get)))
        (bind _output_get (set `self.firstVineOverlap` true))
        (else
          (`KismetSystemLibrary.PrintString` (`KismetStringLibrary.Conv_BoolToString` (stale _output_get_2)))
          (bind _output_get_2 (set `self.firstVineOverlap` false)))))))

(event `self.ReceiveTick`
  (params (DeltaSeconds :type "Float (single-precision)"))
  (bind _startz (`self.startZ`))
  (bind _startz_2 (`self.startZ`))
  (bind _returnvalue (- (`self.startZ`) (`self.LowerHeight`)))
  (bind _returnvalue_2 (- (`self.startZ`) (`self.LowerHeight`)))
  (bind _returnvalue_3 (or (`self.berryMaiOverlap`) (and (`/Game/Blueprints/branch.MaiOverlappingBranch` (`self.firstVine`)) (`/Game/SideScrollerCPP/Blueprints/SideScrollerCharacter2.isClimbing` (`self.Mai`)))))
  (`|ExecutionSequence`
    (:`then_0`
      ;[1 1 1] Check if Mai is on Flower Bud, set lowering & raising
      (if _returnvalue_3
        (if (`KismetMathLibrary.InRange_FloatFloat` (.z (`self.K2_GetActorLocation`)) (- _startz 2.0) _startz)
          (if _returnvalue_3
            (set `self.LowerBerry` true)
            (set `self.RiseBerry` false)
            (else
              (set `self.LowerBerry` false)
              (set `self.RiseBerry` false)))
          (elif (`KismetMathLibrary.InRange_FloatFloat` (.z (`self.K2_GetActorLocation`)) _returnvalue (+ _returnvalue 2.0))
            (set `self.LowerBerry` false)))
        (elif (`KismetMathLibrary.InRange_FloatFloat` (.z (`self.K2_GetActorLocation`)) _returnvalue_2 (+ _returnvalue_2 2.0))
          (set `self.RiseBerry` true)
          (elif (`KismetMathLibrary.InRange_FloatFloat` (.z (`self.K2_GetActorLocation`)) (- _startz_2 2.0) _startz_2)
            (set `self.RiseBerry` false)))))
    (:`then_1`
      ;[1 1 1] Lowering Bud & Branch
      (if (or (`self.berryMaiOverlap`) (and (`/Game/Blueprints/branch.MaiOverlappingBranch` (`self.firstVine`)) (`/Game/SideScrollerCPP/Blueprints/SideScrollerCharacter2.isClimbing` (`self.Mai`))))
        (if (`self.LowerBerry`)
          (`self.K2_AddActorWorldOffset` (`KismetMathLibrary.MakeVector` 0.0 0.0 -2.0))
          (`self.K2_AddActorWorldRotation` (`self.Branch`) (`KismetMathLibrary.MakeRotator` 0.035 0.0) false false)
          (`self.K2_AddActorWorldOffset` (`self.Branch`) (`KismetMathLibrary.MakeVector` 0.0 0.3) false false))))
    (:`then_2`
      ;[1 1 1] Rising Bud & Branch
      (if _returnvalue_3
        _
        (elif (`self.RiseBerry`)
          (`self.K2_AddActorWorldOffset` (`KismetMathLibrary.MakeVector` 0.0 0.0 2.0))
          (`self.K2_AddActorWorldRotation` (`self.Branch`) (`KismetMathLibrary.MakeRotator` -0.035 0.0) false false)
          (`self.K2_AddActorWorldOffset` (`self.Branch`) (`KismetMathLibrary.MakeVector` 0.0 -0.3) false false))))
    (:`then_3`
      ;[1 1 1] If Mai gets off Bud, Rise Bud & Branch
      (if _returnvalue_3
        _
        (elif (`KismetMathLibrary.InRange_FloatFloat` (.z (`self.K2_GetActorLocation`)) (- (`self.startZ`) (`self.LowerHeight`)) (- (`self.startZ`) 2.0))
          (`self.K2_AddActorWorldOffset` (`KismetMathLibrary.MakeVector` 0.0 0.0 2.0))
          (`self.K2_AddActorWorldRotation` (`self.Branch`) (`KismetMathLibrary.MakeRotator` -0.035 0.0) false false)
          (`self.K2_AddActorWorldOffset` (`self.Branch`) (`KismetMathLibrary.MakeVector` 0.0 -0.3) false false))))
    (:`then_4`
      (bind _outactors (`GameplayStatics.GetAllActorsOfClass` "/Game/mergedVine.mergedVine_C"))
      (for _array_element _outactors
        _)
      (bind _staticmeshcomponent (`StaticMeshActor.StaticMeshComponent` _array_element))
      (if (`SceneComponent.IsVisible` _staticmeshcomponent)
        (set `PrimitiveComponent.bGenerateOverlapEvents` true _staticmeshcomponent)))))

(fn `UserConstructionScript`)
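; Cuttable log actor that can shrink and glow before removing itself, driven by two flags that this graph polls on Tick.
; ShouldShrink steps the actor's X and Z scale down each frame until X reaches a minimum.
; IsGlow takes priority, starting a timeline that clears the flag, animates the mesh material's Blend parameter and destroys the actor when finished.
; BeginPlay creates the dynamic material instance for that effect.
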(event `self.ReceiveBeginPlay`
  (bind _staticmeshcomponent (`self.StaticMeshComponent`))
  (`PrimitiveComponent.CreateDynamicMaterialInstance` _staticmeshcomponent 0 (`PrimitiveComponent.GetMaterial` _staticmeshcomponent 0))
  (`KismetSystemLibrary.PrintString` ""))

(event `self.ReceiveTick`
  (params (DeltaSeconds :type "Float (single-precision)"))
  (bind _returnvalue (`self.GetActorScale3D`))
  (if (`self.IsGlow`)
    (`KismetSystemLibrary.PrintString` "ISGLOW")
    (bind (_direction _blend) (`Timeline|Timeline_0`)
      (:`Update`
        (set `self.IsGlow` false)
        (`MeshComponent.SetScalarParameterValueOnMaterials` (`self.StaticMeshComponent`) "Blend" _blend))
      (:`Finished`
        (`self.K2_DestroyActor`)))
    (elif (`self.shouldShrink`)
      (if (> (.x _returnvalue) 9.75)
        (`self.SetActorScale3D` (- _returnvalue (0.25 0.0 0.25)))))))

(fn `UserConstructionScript`)
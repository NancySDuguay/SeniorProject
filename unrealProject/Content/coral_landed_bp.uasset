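; Coral landing Blueprint that tells the side-scroller player character when it is touching the ground.
; Actor begin and end overlap events check that the other actor's class is exactly SideScrollerCharacter2, cast to it, and set its IsTouchingGround flag true on entry and false on exit.
; BeginPlay, Tick and the construction script are empty, so all behavior is driven by overlaps.
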(event `self.ReceiveActorBeginOverlap`
  (params (OtherActor :type "Actor Object Reference"))
  (if (== (`GameplayStatics.GetObjectClass` OtherActor) "/Game/SideScrollerCPP/Blueprints/SideScrollerCharacter2.SideScrollerCharacter2_C")
    (bind _asside_scroller_character_2 (cast `/Game/SideScrollerCPP/Blueprints/SideScrollerCharacter2` OtherActor))
    (set `/Game/SideScrollerCPP/Blueprints/SideScrollerCharacter2.isTouchingGround` true _asside_scroller_character_2)))

(event `self.ReceiveActorEndOverlap`
  (params (OtherActor :type "Actor Object Reference"))
  (if (== (`GameplayStatics.GetObjectClass` OtherActor) "/Game/SideScrollerCPP/Blueprints/SideScrollerCharacter2.SideScrollerCharacter2_C")
    (bind _asside_scroller_character_2 (cast `/Game/SideScrollerCPP/Blueprints/SideScrollerCharacter2` OtherActor))
    (set `/Game/SideScrollerCPP/Blueprints/SideScrollerCharacter2.isTouchingGround` false _asside_scroller_character_2)))

(fn `UserConstructionScript`)